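; Interactable puzzle door that swings open and moves its lock bar once four cross valves bring Level to exactly 230.
; Interact stores the impact point, and Verificator finds the valve hit via a zero closest-point-on-collision distance.
; Per-valve FlipFlops play or reverse rotation timelines and adjust Level; timeline updates call OpenTheDoor to check the total.
; Turning back is inconsistent: Cross1 leaves Level unchanged, while Cross2 and Cross4 compute 50 minus Level.
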(event Custom|Open%20the%20door
  ;[0.04144 0.6384 0.7406 0.5] Open Doors Système
  (if (== (Variables|Default|GetLevel?) 230)
    (bind (_direction _door_move _lock_move_rot _loock_move_trans) (Timeline|Door Play)
      (:Update
        (Transformation|SetRelativeRotation (Variables|Default|GetMetal_Door) (Math|Rotator|MakeRotator 0.0 0.0 _door_move) false false)
        (Transformation|SetRelativeTransform (Variables|Default|GetLock_bar) (Math|Transform|MakeTransform (Math|Vector|MakeVector _loock_move_trans 1.0 103.0) (Math|Rotator|MakeRotator _lock_move_rot 0.0 0.0) "1.000000,1.000000,1.000000") false false)))))

(event Custom|Verificator
  (bind _impact_point (Variables|Default|GetImpact%20Point))
  (Utilities|FlowControl|Sequence
    (:then_0
      (if (== (.ReturnValue (Collision|GetClosestPointonCollision (Variables|Default|GetCross1) _impact_point "None")) 0.0)
        (Utilities|FlowControl|FlipFlop
          (:A
            (Variables|Default|SetLevel? (+ (Variables|Default|GetLevel?) 50))
            (bind _newtrack_0 (Timeline|Time%20to%20line Play)
              (:Update
                (Transformation|SetRelativeRotation (Variables|Default|GetCross1) (Math|Rotator|MakeRotator 0.0 _newtrack_0 0.0) false false)
                (CallFunction|OpentheDoor))))
          (:B
            (Timeline|Time%20to%20line Reverse)))))
    (:then_1
      (if (== (.ReturnValue (Collision|GetClosestPointonCollision (Variables|Default|GetCross2) _impact_point "None")) 0.0)
        (Utilities|FlowControl|FlipFlop
          (:A
            (Variables|Default|SetLevel? (+ (Variables|Default|GetLevel?) 50))
            (bind _newtrack_0_2 (Timeline|Timeline_0 Play)
              (:Update
                (Transformation|SetRelativeRotation (Variables|Default|GetCross2) (Math|Rotator|MakeRotator 0.0 _newtrack_0_2 0.0) false false)
                (CallFunction|OpentheDoor))))
          (:B
            (Variables|Default|SetLevel? (- 50 (Variables|Default|GetLevel?)))
            (Timeline|Timeline_0 Reverse)))))
    (:then_2
      (if (== (.ReturnValue (Collision|GetClosestPointonCollision (Variables|Default|GetCross3) _impact_point "None")) 0.0)
        (Utilities|FlowControl|FlipFlop
          (:A
            (Variables|Default|SetLevel? (+ (Variables|Default|GetLevel?) 80))
            (bind _newtrack_0_3 (Timeline|Timeline Play)
              (:Update
                (Transformation|SetRelativeRotation (Variables|Default|GetCross3) (Math|Rotator|MakeRotator 0.0 _newtrack_0_3 0.0) false false)
                (CallFunction|OpentheDoor))))
          (:B
            (Variables|Default|SetLevel? (- (Variables|Default|GetLevel?) 80))
            (Timeline|Timeline Reverse)))))
    (:then_3
      (if (== (.ReturnValue (Collision|GetClosestPointonCollision (Variables|Default|GetCross4) _impact_point "None")) 0.0)
        (Utilities|FlowControl|FlipFlop
          (:A
            (Variables|Default|SetLevel? (+ (Variables|Default|GetLevel?) 50))
            (bind _newtrack_0_4 (Timeline|Timeline_1 Play)
              (:Update
                (Transformation|SetRelativeRotation (Variables|Default|GetCross4) (Math|Rotator|MakeRotator 0.0 _newtrack_0_4 0.0) false false)
                (CallFunction|OpentheDoor))))
          (:B
            (Variables|Default|SetLevel? (- 50 (Variables|Default|GetLevel?)))
            (Timeline|Timeline_1 Reverse)))))))

(event EventInteract
  (params (ImpactPoint :type Vector :default "0, 0, 0"))
  ;[0.1862 0.1744 0.9656 0.5] Init
  (Variables|Default|SetImpact%20Point ImpactPoint)
  (CallFunction|Verificator))

(fn ConstructionScript)