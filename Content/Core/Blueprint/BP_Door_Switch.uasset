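; Switch-puzzle door that opens its metal door once five switches are flipped on in the right order (3, 5, 2, 4, 1).
; Interact passes an impact point to Verificator, which finds the hit switch box by zero closest-point distance and toggles that switch's tilt through a FlipFlop.
; Correct flips advance FiveActivate, and the last fires a timeline moving door and lock bar.
; Wrong flips leave progress intact; the reset event is marked unused.
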(event Custom|Open%20the%20door
  ;[0.04144 0.6384 0.7406 0.5] Open Doors Système
  (bind (_direction _door_move _lock_move_rot _loock_move_trans) (Timeline|Door Play)
    (:Update
      (Transformation|SetRelativeRotation (Variables|Default|GetMetal_Door) (Math|Rotator|MakeRotator 0.0 0.0 _door_move) false false)
      (Transformation|SetRelativeTransform (Variables|Default|GetLock_bar) (Math|Transform|MakeTransform (Math|Vector|MakeVector _loock_move_trans 1.0 103.0) (Math|Rotator|MakeRotator _lock_move_rot 0.0 0.0) "1.000000,1.000000,1.000000") false false))))

(event Custom|Verificator
  (bind _impact_point (Variables|Default|GetImpact%20Point))
  (bind _sw1 (Variables|Default|GetSw1))
  (bind _sw2 (Variables|Default|GetSw2))
  (bind _sw3 (Variables|Default|GetSw3))
  (bind _sw4 (Variables|Default|GetSw4))
  (bind _sw5 (Variables|Default|GetSw5))
  ;[0.7406 0 0.02961 0.5] Systeme code
  (Utilities|FlowControl|Sequence
    (:then_0
      (if (== (.ReturnValue (Collision|GetClosestPointonCollision (Variables|Default|GetBox_1) _impact_point "None")) 0.0)
        (Utilities|FlowControl|FlipFlop
          (:A
            (Transformation|SetRelativeRotation _sw1 "0.000000,0.000000,50.000000" false false)
            (if (== (Variables|Default|GetFiveActivate?) 1234)
              (CallFunction|OpentheDoor)))
          (:B
            (Transformation|SetRelativeRotation _sw1 "0, 0, 0" false false)))))
    (:then_1
      (if (== (.ReturnValue (Collision|GetClosestPointonCollision (Variables|Default|GetBox_2) _impact_point "None")) 0.0)
        (Utilities|FlowControl|FlipFlop
          (:A
            (Transformation|SetRelativeRotation _sw2 "0.000000,0.000000,50.000000" false false)
            (if (== (Variables|Default|GetFiveActivate?) 12)
              (Variables|Default|SetFiveActivate? 123)))
          (:B
            (Transformation|SetRelativeRotation _sw2 "0, 0, 0" false false)))))
    (:then_2
      (if (== (.ReturnValue (Collision|GetClosestPointonCollision (Variables|Default|GetBox_3) _impact_point "None")) 0.0)
        (Utilities|FlowControl|FlipFlop
          (:A
            (Transformation|SetRelativeRotation _sw3 "0.000000,0.000000,50.000000" false false)
            (if (== (Variables|Default|GetFiveActivate?) 0)
              (Variables|Default|SetFiveActivate? 1)))
          (:B
            (Transformation|SetRelativeRotation _sw3 "0, 0, 0" false false)))))
    (:then_3
      (if (== (.ReturnValue (Collision|GetClosestPointonCollision (Variables|Default|GetBox_4) _impact_point "None")) 0.0)
        (Utilities|FlowControl|FlipFlop
          (:A
            (Transformation|SetRelativeRotation _sw4 "0.000000,0.000000,50.000000" false false)
            (if (== (Variables|Default|GetFiveActivate?) 123)
              (Variables|Default|SetFiveActivate? 1234)))
          (:B
            (Transformation|SetRelativeRotation _sw4 "0, 0, 0" false false)))))
    (:then_4
      (if (== (.ReturnValue (Collision|GetClosestPointonCollision (Variables|Default|GetBox_5) _impact_point "None")) 0.0)
        (Utilities|FlowControl|FlipFlop
          (:A
            (Transformation|SetRelativeRotation _sw5 "0.000000,0.000000,50.000000" false false)
            (if (== (Variables|Default|GetFiveActivate?) 1)
              (Variables|Default|SetFiveActivate? 12)))
          (:B
            (Transformation|SetRelativeRotation _sw5 "0, 0, 0" false false)))))))

(event Custom|reset
  ;[0 0 0 0.5] Not used system cause time
  (Transformation|SetRelativeRotation (Variables|Default|GetSw2) "0, 0, 0" false false))

(event EventInteract
  (params (ImpactPoint :type Vector :default "0, 0, 0"))
  ;[0.1862 0.1744 0.9656 0.5] Init
  (Variables|Default|SetImpact%20Point ImpactPoint)
  (CallFunction|Verificator))

(fn ConstructionScript)